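; Blueprint implementation of the One Euro filter, an adaptive low-pass filter that smooths a single float signal.
; XOneEuroFilter sets up two exponential low-pass filters, one for the value and one for its derivative.
; XOEFfilter estimates speed and raises the value filter's cutoff with it, trading jitter against lag.
; The derivative filter's initialized flag is never set true, so speed passes through unsmoothed.
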(event EventBeginPlay)

(event EventTick
  (params (DeltaSeconds :type Float%20%28single-precision%29)))

(fn XLPFsetAlfa
  (params (alfa :type Float%20%28single-precision%29))
  (if (< alfa 0.0)
    (Variables|Default|SetxLPFa 0.0)
    (elif (> alfa 1.0)
      (Variables|Default|SetxLPFa 1.0)
      (else
        (Variables|Default|SetxLPFa alfa)))))

(fn DxLPFsetAlfa
  (params (alfa :type Float%20%28single-precision%29))
  (if (< alfa 0.0)
    (Variables|Default|SetdxLPFa 0.0)
    (elif (> alfa 1.0)
      (Variables|Default|SetdxLPFa 1.0)
      (else
        (Variables|Default|SetdxLPFa alfa)))))

(fn XLowPassFilter
  (params (alfa :type Float%20%28single-precision%29) (initval :type Float%20%28single-precision%29))
  (bind _output_get (Variables|Default|SetxLPFy initval))
  (Variables|Default|SetxLPFs _output_get)
  (CallFunction|XLPFsetAlfa alfa)
  (Variables|Default|SetxLPFinitialized false))

(fn DxLowPassFilter
  (params (alfa :type Float%20%28single-precision%29) (initval :type Float%20%28single-precision%29))
  (bind _output_get (Variables|Default|SetdxLPFy initval))
  (Variables|Default|SetdxLPFs _output_get)
  (CallFunction|DxLPFsetAlfa alfa)
  (Variables|Default|SetdxLPFinitialized false))

(fn XLPFfilter
  (params (value :type Float%20%28single-precision%29))
  (bind _xlpfa (Variables|Default|GetxLPFa))
  (if (Variables|Default|GetxLPFinitialized)
    (LocalVariables|Setresult (+ (* _xlpfa value) (* (- 1.0 _xlpfa) (Variables|Default|GetxLPFs))))
    (else
      (LocalVariables|Setresult value)
      (Variables|Default|SetxLPFinitialized true)))
  (Variables|Default|SetxLPFy value)
  (bind _output_get (Variables|Default|SetxLPFs (LocalVariables|Getresult)))
  (return _output_get))

(fn DxLPFfilter
  (params (value :type Float%20%28single-precision%29))
  (bind _dxlpfa (Variables|Default|GetdxLPFa))
  (if (Variables|Default|GetdxLPFinitialized)
    (LocalVariables|Setresult (+ (* _dxlpfa value) (* (- 1.0 _dxlpfa) (Variables|Default|GetdxLPFs))))
    (else
      (LocalVariables|Setresult value)))
  (Variables|Default|SetdxLPFy value)
  (bind _output_get (Variables|Default|SetdxLPFs (LocalVariables|Getresult)))
  (return _output_get))

(fn XLPFfilterwithAlfa
  (params (value :type Float%20%28single-precision%29) (alfa :type Float%20%28single-precision%29))
  (CallFunction|XLPFsetAlfa alfa)
  (bind _dlpfresult (CallFunction|XLPFfilter value))
  (return _dlpfresult))

(fn DxLPFfilterwithAlfa
  (params (value :type Float%20%28single-precision%29) (alfa :type Float%20%28single-precision%29))
  (CallFunction|DxLPFsetAlfa alfa)
  (bind _dxlpfresult (CallFunction|DxLPFfilter value))
  (return _dxlpfresult))

(fn XOEFalfa
  (params (cutoff :type Float%20%28single-precision%29) (frequency :type Float%20%28single-precision%29))
  (return (/ 1.0 (+ (/ (/ 1.0 (Math|Float|MultiplybyPi (* cutoff 2.0))) (/ 1.0 frequency)) 1.0))))

(fn XOneEuroFilter
  (params (freq :type Float%20%28single-precision%29) (mincutoff :type Float%20%28single-precision%29) (beta :type Float%20%28single-precision%29) (dcutoff :type Float%20%28single-precision%29))
  (Variables|Default|SetxLPFinitialized false)
  (Variables|Default|SetdxLPFinitialized false)
  (bind _output_get (Variables|Default|SetxOEFfreq freq))
  (Variables|Default|SetxOEFmincutoff mincutoff)
  (Variables|Default|SetxOEFbeta beta)
  (Variables|Default|SetxOEFdcutoff dcutoff)
  (bind _ret (CallFunction|XOEFalfa mincutoff _output_get))
  (CallFunction|XLowPassFilter _ret 0.0)
  (bind _ret_2 (CallFunction|XOEFalfa dcutoff _output_get))
  (CallFunction|DxLowPassFilter _ret_2 0.0))

(fn XOEFfilter
  (params (value :type Float%20%28single-precision%29))
  (if (Variables|Default|GetxLPFinitialized)
    (LocalVariables|Setdvalue (* (- value (Variables|Default|GetxLPFy)) (Variables|Default|GetxOEFfreq)))
    (else
      (LocalVariables|Setdvalue 0.0)))
  ;[1 1 1] edvalue = dxLPFfilterWithAlfa(dvalue, xOEFalfa(xOEFdcutoff, xOEFfreq))
  (bind _ret (CallFunction|XOEFalfa (Variables|Default|GetxOEFdcutoff) (Variables|Default|GetxOEFfreq)))
  (bind _ret_2 (CallFunction|DxLPFfilterwithAlfa (LocalVariables|Getdvalue) _ret))
  (LocalVariables|Setedvalue _ret_2)
  ;[1 1 1] cutoff = xOEFmincutoff + xOEFbeta * abs(edvalue);
  (LocalVariables|Setcutoff (+ (Variables|Default|GetxOEFmincutoff) (* (Variables|Default|GetxOEFbeta) (Math|Float|Absolute(Float) (LocalVariables|Getedvalue)))))
  ;[1 1 1] xLPFfilterWithAlfa(value, xOEFalfa(cutoff, xOEFfreq))
  (bind _ret_3 (CallFunction|XOEFalfa (LocalVariables|Getcutoff) (Variables|Default|GetxOEFfreq)))
  (bind _ret_4 (CallFunction|XLPFfilterwithAlfa value _ret_3))
  (return _ret_4))